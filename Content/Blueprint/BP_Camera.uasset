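; BP_Camera is a rail camera that follows the player along a spline.
; On BeginPlay it makes itself the view target of the first player controller.
; Each Tick it finds the spline point closest to the player character and smoothly interpolates the Camera component's world position toward it with VInterpTo.
; Only the camera's location is updated, never its rotation.
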(event EventBeginPlay
  ;[1 1 1] Set la camera
  (Game|Player|SetViewTargetwithBlend (Game|GetPlayerController 0) self 0.0 "VTBlend_Linear" 0.0 false))

(event EventTick
  (params (DeltaSeconds :type Float%20%28single-precision%29))
  (bind _camera (Variables|Default|GetCamera))
  ;[1 1 1] Déplace la camera de sorte à suivre le player en fonction de la spline
  (Transformation|SetWorldLocation _camera (Math|Interpolation|VInterpTo (Transformation|GetWorldLocation _camera) (Spline|FindLocationClosesttoWorldLocation (Variables|Default|GetSpline) (Transformation|GetActorLocation (Game|GetPlayerCharacter 0)) "World") (Utilities|Time|GetWorldDeltaSeconds) 2.0) false false))

(fn ConstructionScript)