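; BP_FireFlower is a Fire Flower collectable that acts as a coin pickup for BP_Mario.
; BeginPlay stores the start location and sets the bob timeline's play rate and the rotation speed.
; The timeline, noted as auto-looping, lerps the flower mesh vertically, feeding the saved world location into SetRelativeLocation.
; Overlap by Mario plays a sound, adds Bonus coins through the GameInstance, refreshes the player UI and destroys the actor.
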(event Collision|EventActorBeginOverlap
  (params (OtherActor :type Actor%20Object%20Reference))
  ;[1 1 1] Gestion de la collision du joueur avec une pièce et compte le nb de pièce
  (Utilities|Casting|CastToBP_Mario OtherActor)
  (Audio|SpawnSound2D "/Game/Audio/Coin_Collect_-_Sound_Effect.Coin_Collect_-_Sound_Effect" 1.0 1.0 0.8 0)
  (bind _asgi_mario (CallFunction|GetGI))
  (Default|AddCoin _asgi_mario (Variables|Default|Getbonus))
  (bind _aspc_mario (CallFunction|GetPC))
  (Default|UpdateCoin (Variables|/Game/system/PC_Mario.PC_Mario_C|GetUIPlayerRef _aspc_mario))
  (Actor|DestroyActor))

(event EventBeginPlay
  ;[1 1 1] Sauvegarde de la position initial d'une pièce
  (Variables|Default|SetpositionInitial (Transformation|GetActorLocation))
  ;[1 1 1] Facteur multiplicateur de la vitesse de découlement de la timeline
  (Components|Timeline|SetPlayRate (Variables|Default|GetTimeline) (Variables|Default|Getrate))
  ;[1 1 1] Vitesse de rotation
  (Variables|/Script/Engine.RotatingMovementComponent|SetRotationRate (Variables|Default|GetRotatingMovement) (Math|Rotator|MakeRotator 0.0 0.0 (Variables|Default|GetRotationRate))))

(fn ConstructionScript)