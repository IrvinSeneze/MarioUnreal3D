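; BP_Mario is a player character for Mario-style movement along its forward axis, driven by Enhanced Input.
; Sprint raises walk speed and eases it back through a timeline on release, while Tick flips the mesh to match velocity direction.
; Jump scales its launch velocity by trigger time within clamped limits, after a short delay.
; Crouch becomes a downward dive impulse in midair, blocking movement until the input completes.
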(event Input|EnhancedActionEvents|EnhancedInputActionINP_Sprint
  (params (ActionValue :type Boolean) (ElapsedSeconds :type Float%20%28double-precision%29) (TriggeredSeconds :type Float%20%28double-precision%29) (InputAction :type Input%20Action%20Object%20Reference :default "/Game/Blueprint/mario/Inputs/INP_Sprint.INP_Sprint"))
  (bind _charactermovement (Variables|Character|GetCharacterMovement))
  ;[1 1 1] Permet au joueur de sprint
  (:Started
    (Variables|Default|SetIsSprinting true)
    (Variables|/Script/Engine.CharacterMovementComponent|SetMaxWalkSpeed _charactermovement 1e+03)
    (bind _stopsprinting (Timeline|Timeline Stop)
      (:Update
        (Variables|/Script/Engine.CharacterMovementComponent|SetMaxWalkSpeed _charactermovement _stopsprinting))))
  (:Canceled
    (Variables|Default|SetIsSprinting false :!label _label)
    (Timeline|Timeline PlayFromStart))
  (:Completed
    (goto _label)))

(event Input|EnhancedActionEvents|EnhancedInputActionINP_Move
  (params (ActionValue :type Vector%202D%20Structure) (ElapsedSeconds :type Float%20%28double-precision%29) (TriggeredSeconds :type Float%20%28double-precision%29) (InputAction :type Input%20Action%20Object%20Reference :default "/Game/Blueprint/mario/Inputs/INP_Move.INP_Move"))
  ;[1 1 1] Mouvement
  (if (Variables|Default|GetCanMove)
    (Pawn|Input|AddMovementInput (Transformation|GetActorForwardVector) (.x ActionValue) false)))

(event Input|EnhancedActionEvents|EnhancedInputActionINP_Jump
  (params (ActionValue :type Boolean) (ElapsedSeconds :type Float%20%28double-precision%29) (TriggeredSeconds :type Float%20%28double-precision%29) (InputAction :type Input%20Action%20Object%20Reference :default "/Game/Blueprint/mario/Inputs/INP_Jump.INP_Jump"))
  (bind _charactermovement (Variables|Character|GetCharacterMovement))
  (bind _jumpforce (Variables|Default|GetJumpForce))
  (bind _returnvalue (* TriggeredSeconds _jumpforce))
  ;[1 1 1] Sauter
  (:Triggered
    (if (not (AI|Components|NavMovement|IsCrouching (Variables|Character|GetCharacterMovement)))
      (Variables|Default|SetIsJumping true)
      (Utilities|FlowControl|Delay 0.2)
      (if (not (> _returnvalue 1.5e+03))
        (if (not (< _returnvalue 7.5e+02))
          (Variables|/Script/Engine.CharacterMovementComponent|SetJumpZVelocity _charactermovement _returnvalue)
          (else
            (Variables|/Script/Engine.CharacterMovementComponent|SetJumpZVelocity _charactermovement 7.5e+02)))
        (else
          (Variables|/Script/Engine.CharacterMovementComponent|SetJumpZVelocity _charactermovement 1.5e+03)))
      (Character|Jump)
      (Variables|Default|SetIsJumping false)))
  (:Canceled
    (Variables|Default|SetIsJumping false)
    (Character|StopJumping)))

(event Input|EnhancedActionEvents|EnhancedInputActionINP_Crouch
  (params (ActionValue :type Boolean) (ElapsedSeconds :type Float%20%28double-precision%29) (TriggeredSeconds :type Float%20%28double-precision%29) (InputAction :type Input%20Action%20Object%20Reference :default "/Game/Blueprint/mario/Inputs/INP_Crouch.INP_Crouch"))
  ;[1 1 1] Accroupi et Diving
  (:Started
    (if (AI|Components|NavMovement|IsFalling (Variables|Character|GetCharacterMovement))
      (if (not (Variables|Default|GetIsDiving))
        (Physics|AddImpulse (Variables|Character|GetCharacterMovement) "0.000000,0.000000,-1500.000000" true)
        (Variables|Default|SetIsDiving true)
        (Variables|Default|SetCanMove false))
      (else
        (Character|Crouch))))
  (:Completed
    (Character|UnCrouch)
    (Variables|Default|SetIsDiving false)
    (Variables|Default|SetCanMove true)))

(event EventBeginPlay
  ;[1 1 1] Innitialisation du mapping context
  (bind _aspc_mario (Utilities|Casting|CastToPC_Mario (Pawn|GetController)))
  (Utilities|IsValid (PlayerController|LocalPlayerSubsystems|GetEnhancedInputLocalPlayerSubsystem _aspc_mario)
    (:Is%20Valid
      (Input|AddMappingContext (PlayerController|LocalPlayerSubsystems|GetEnhancedInputLocalPlayerSubsystem _aspc_mario) "/Game/Blueprint/mario/Inputs/IMC_Mario.IMC_Mario" 0 "(bIgnoreAllPressedKeysUntilRelease=True,bForceImmediately=False,bNotifyUserSettings=False)"))))

(event EventTick
  (params (DeltaSeconds :type Float%20%28single-precision%29))
  (bind _mesh (Variables|Character|GetMesh))
  ;[1 1 1] Changer la direction de l'animation
  (Math|Float|CompareFloat (Math|Vector|DotProduct (Transformation|GetVelocity) (Transformation|GetActorForwardVector)) 0.0
    (:>
      (Transformation|SetRelativeRotation _mesh "0.000000,-90.000000,0.000000" false false))
    (:<
      (Transformation|SetRelativeRotation _mesh "0.000000,90.000000,0.000000" false false))))

(fn ConstructionScript)