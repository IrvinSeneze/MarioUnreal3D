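; BP_Goomba is a Goomba enemy that Mario kills by landing on its head.
; Head overlap plays a squash Timeline, makes a non-diving Mario jump, then destroys the actor; body overlap blocks the kill.
; A second Timeline holds back-and-forth movement logic that lerps along a Movement offset and flips the body at each end, but nothing in the graph plays it.
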(event OnComponentBeginOverlap(HeadCapsule)
  (params (OverlappedComponent :type Primitive%20Component%20Object%20Reference) (OtherActor :type Actor%20Object%20Reference) (OtherComp :type Primitive%20Component%20Object%20Reference) (OtherBodyIndex :type Integer) (bFromSweep :type Boolean) (SweepResult :type Hit%20Result%20Structure%20%28by%20ref%29))
  (bind _initialscale (Variables|Default|GetInitialScale))
  (bind _asbp_mario (Utilities|Casting|CastToBP_Mario OtherActor))
  (if (Variables|Default|GetcanBeKilled)
    ;[1 1 1] Gère le rescale du gomba pour faire un effet d'ecrassement
    (bind _size (Timeline|Timeline Play)
      (:Update
        (Transformation|SetRelativeScale3D (Variables|Default|GetBody) (Math|Vector|Lerp(Vector) _initialscale (+ _initialscale "0.000000,-15.000000,0.000000") _size))
        (Utilities|FlowControl|Delay 0.2)
        ;[1 1 1] Saut de mario après avoir tuer l'ennemie
        (if (not (Variables|/Game/Blueprint/mario/BP_Mario.BP_Mario_C|GetIsDiving _asbp_mario))
          (Character|Jump _asbp_mario)
          ;[1 1 1] Destruction de l'ennemie
          (Utilities|FlowControl|Delay 0.2))
        (Actor|DestroyActor)))))

(event OnComponentBeginOverlap(BodyCapsule)
  (params (OverlappedComponent :type Primitive%20Component%20Object%20Reference) (OtherActor :type Actor%20Object%20Reference) (OtherComp :type Primitive%20Component%20Object%20Reference) (OtherBodyIndex :type Integer) (bFromSweep :type Boolean) (SweepResult :type Hit%20Result%20Structure%20%28by%20ref%29))
  ;[1 1 1] Permet de ne pas tuer le goomba depuis son corp au lieu de sa tête
  (Utilities|Casting|CastToBP_Mario OtherActor)
  (Variables|Default|SetcanBeKilled false))

(event OnComponentEndOverlap(BodyCapsule)
  (params (OverlappedComponent :type Primitive%20Component%20Object%20Reference) (OtherActor :type Actor%20Object%20Reference) (OtherComp :type Primitive%20Component%20Object%20Reference) (OtherBodyIndex :type Integer))
  ;[1 1 1] Permet de ne pas tuer le goomba depuis son corp au lieu de sa tête
  (Utilities|Casting|CastToBP_Mario OtherActor)
  (Variables|Default|SetcanBeKilled true))

(event EventBeginPlay
  ;[1 1 1] Set la valeur de scale initial et le play rate de l'animation
  (Variables|Default|SetInitialScale (Variables|/Script/Engine.SceneComponent|GetRelativeScale3D (Variables|Default|GetBody)))
  (Variables|Default|SetInitialLocation (Variables|/Script/Engine.SceneComponent|GetRelativeLocation (Variables|Default|GetGoomba)))
  (Components|Timeline|SetPlayRate (Variables|Default|GetTimeline) (Variables|Default|GetSpeedRate))
  (Components|Timeline|SetPlayRate (Variables|Default|GetMovementTimeline) (/ 1.0 (/ (.x (Variables|Default|GetMovement)) 2e+02))))

(fn ConstructionScript)