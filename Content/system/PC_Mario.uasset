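; PC_Mario is the player controller for a Mario game, managing the player UI and the game over screen.
; On BeginPlay it creates the UI_Player widget, keeps a reference to it, and switches to game-only input with a hidden cursor.
; Its gameOver event shows the UI_GameOver widget and cursor, disables input on the player character, and focuses UI-only input on that widget.
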(event Custom|gameOver
  (bind _self self)
  ;[1 1 1] Affichage du game over, affichage de la souris et disable input du joueur
  (bind _returnvalue (UserInterface|CreateWidget "/Game/UI/UI_GameOver.UI_GameOver_C" self))
  (UserInterface|Viewport|AddtoViewport _returnvalue 0)
  (Variables|Default|SetbShowMouseCursor true)
  (Input|DisableInput (Game|GetPlayerCharacter 0) _self)
  (Input|SetInputModeUIOnly _self _returnvalue "DoNotLock" false))

(event EventBeginPlay
  (bind _self self)
  ;[1 1 1] Création et affichage de l'interface graphique
  (bind _returnvalue (UserInterface|CreateWidget "/Game/UI/UI_Player.UI_Player_C" _self))
  (bind _output_get (Variables|Default|SetUIPlayerRef _returnvalue))
  (UserInterface|Viewport|AddtoViewport _output_get 0)
  ;[1 1 1] Activation du mode de jeu
  (Input|SetInputModeGameOnly _self false)
  (Variables|Default|SetbShowMouseCursor false))

(fn ConstructionScript)